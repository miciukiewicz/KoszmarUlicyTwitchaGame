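; Halloween skeleton prop with a configurable mount (none, stand or hanger) and bone color, both applied in the construction script.
; When ShouldMove is set, a looping timer periodically kicks one bone of the Cube component with a random, always-positive velocity impulse and plays the bone-rattle cue.
; The first player character entering the trigger box also plays that cue, without applying an impulse.
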(event OnComponentBeginOverlap(Box)
  (params (OverlappedComponent :type Primitive%20Component%20Object%20Reference) (OtherActor :type Actor%20Object%20Reference) (OtherComp :type Primitive%20Component%20Object%20Reference) (OtherBodyIndex :type Integer) (bFromSweep :type Boolean) (SweepResult :type Hit%20Result%20Structure%20%28by%20ref%29))
  (if (== OtherActor (Game|GetPlayerCharacter 0))
    (Audio|Components|Audio|Play (Variables|Default|GetSkeletonBones_Cue) 0.0)))

(event Custom|MoveSkeleton
  (Physics|AddImpulse (Variables|Default|GetCube) (Math|Vector|MakeVector (Math|Random|RandomFloatinRange 1e+03 5e+03) (Math|Random|RandomFloatinRange 1e+03 5e+03) (Math|Random|RandomFloatinRange 1e+03 5e+03)) "Bone_016" true)
  (Audio|Components|Audio|Play (Variables|Default|GetSkeletonBones_Cue) 0.0))

(event EventBeginPlay
  (if (Variables|Default|GetshouldMove)
    (Utilities|Time|SetTimerbyFunctionName 0 "MoveSkeleton" 5.0 true)))

(fn ConstructionScript
  (bind _sm_skeletonhanger (Variables|Default|GetSM_SkeletonHanger))
  (bind _sm_skeletonstand (Variables|Default|GetSM_SkeletonStand))
  (bind _sm_skeleton (Variables|Default|GetSM_Skeleton))
  (Utilities|FlowControl|Sequence
    (:then_0
      (switch Utilities|FlowControl|Switch|SwitchonSkeletonType (Variables|Default|GetplacementType)
        (:NewEnumerator0
          (Rendering|SetVisibility _sm_skeletonhanger false false))
        (:NewEnumerator1
          (Rendering|SetVisibility _sm_skeletonstand true false)
          (Rendering|SetVisibility _sm_skeletonhanger false false))
        (:NewEnumerator2
          (Rendering|SetVisibility _sm_skeletonhanger true false)
          (Rendering|SetVisibility _sm_skeletonstand false false))))
    (:then_1
      (switch Utilities|FlowControl|Switch|SwitchonskeletonColor (Variables|Default|GetskeletonColor)
        (:NewEnumerator0
          (Rendering|Material|SetMaterial _sm_skeleton 0 "/Game/Halloween/Props/Other/Skeleton/Textures/SkeletonDefault_Mat.SkeletonDefault_Mat"))
        (:NewEnumerator1
          (Rendering|Material|SetMaterial _sm_skeleton 0 "/Game/Halloween/Props/Other/Skeleton/Textures/SkeletonWhite_Mat.SkeletonWhite_Mat"))
        (:NewEnumerator2
          (Rendering|Material|SetMaterial _sm_skeleton 0 "/Game/Halloween/Props/Other/Skeleton/Textures/SkeletonRed_Mat.SkeletonRed_Mat"))
        (:NewEnumerator3
          (Rendering|Material|SetMaterial _sm_skeleton 0 "/Game/Halloween/Props/Other/Skeleton/Textures/SkeletonGreen_Mat.SkeletonGreen_Mat"))
        (:NewEnumerator4
          (Rendering|Material|SetMaterial _sm_skeleton 0 "/Game/Halloween/Props/Other/Skeleton/Textures/SkeletonBlue_Mat.SkeletonBlue_Mat"))))))