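; Halloween graveyard prop that builds one of six grave variants from GraveType, each with its own headstone or tomb and decorations.
; The construction script reveals that variant's components, then randomizes flower scale, yaw, mesh and material, plus candle yaw, mesh and color.
; The randomness is unseeded, so decorations reroll whenever construction reruns.
; BeginPlay disables collision on both long tombs for the first two types, which never show them.
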(event EventBeginPlay
  (switch int (Variables|Default|GetgraveType)
    (:0
      _)
    (:1
      _))
  (Collision|SetCollisionEnabled (Variables|Default|GetTombLong1) "NoCollision"))

(event Collision|EventActorBeginOverlap
  (params (OtherActor :type Actor%20Object%20Reference)))

(event EventTick
  (params (DeltaSeconds :type Float%20%28single-precision%29)))

(fn ConstructionScript
  (bind _tomblong1 (Variables|Default|GetTombLong1))
  (bind _tomblong2 (Variables|Default|GetTombLong2))
  (Utilities|FlowControl|Sequence
    (:then_0
      (switch int (Variables|Default|GetgraveType)
        (:0
          (Rendering|SetVisibility (Variables|Default|GetDefaultTomb) true false)
          (Rendering|SetVisibility (Variables|Default|Get2Flowers_0-1) true false :!label _label))
        (:1
          (Rendering|SetVisibility (Variables|Default|GetCross) true false)
          (goto _label))
        (:2
          (Rendering|SetVisibility _tomblong1 true false)
          (Rendering|SetVisibility (Variables|Default|Get1Candle_2-3) true false :!label _label_2))
        (:3
          (Rendering|SetVisibility _tomblong1 true false)
          (goto _label_2))
        (:4
          (Rendering|SetVisibility _tomblong2 true false)
          (Rendering|SetVisibility (Variables|Default|Get1Flowers_4-5) true false :!label _label_3))
        (:5
          (Rendering|SetVisibility _tomblong2 true false)
          (goto _label_3))))
    (:then_1
      (CallFunction|SetRandomFlowers (Variables|Default|Get1Flowers_0-1))
      (CallFunction|SetRandomFlowers (Variables|Default|Get3Flowers_0-1))
      (CallFunction|SetRandomFlowers (Variables|Default|Get2Flowers_4-5))
      (CallFunction|SetRandomFlowers (Variables|Default|Get3Flowers_4-5))
      (CallFunction|SetRandomFlowers (Variables|Default|Get1Flowers_4-5))
      (CallFunction|SetRandomFlowers (Variables|Default|Get2Flowers_0-1)))
    (:then_2
      (CallFunction|SetRandomCandle (Variables|Default|Get1Candle_4-5))
      (CallFunction|SetRandomCandle (Variables|Default|Get3Candle_2-3))
      (CallFunction|SetRandomCandle (Variables|Default|Get3Candle_4-5))
      (CallFunction|SetRandomCandle (Variables|Default|Get2Candle_0-1))
      (CallFunction|SetRandomCandle (Variables|Default|Get2Candle_2-3))
      (CallFunction|SetRandomCandle (Variables|Default|Get1Candle_0-1))
      (CallFunction|SetRandomCandle (Variables|Default|Get1Candle_2-3))
      (CallFunction|SetRandomCandle (Variables|Default|Get2Candle_4-5)))))

(fn SetRandomFlowers
  (params (Mesh :type Static%20Mesh%20Component%20Object%20Reference))
  (bind _returnvalue (Math|Random|RandomFloatinRange 0.9 1.3))
  (Transformation|SetRelativeScale3D Mesh (Math|Vector|MakeVector _returnvalue _returnvalue _returnvalue))
  (Transformation|SetRelativeRotation Mesh (Math|Rotator|MakeRotator 0.0 0.0 (Math|Random|RandomFloatinRange 0.0 359.0)) false false)
  (switch int (Math|Random|RandomIntegerinRange 0 1)
    (:0
      (Components|StaticMesh|SetStaticMesh Mesh "/Game/Halloween/Props/Graveyard/Flowers/SM_Flowers_1.SM_Flowers_1")
      (switch int (Math|Random|RandomIntegerinRange 0 1)
        (:0
          (Rendering|Material|SetMaterial Mesh 0 "/Game/Halloween/Props/Graveyard/Flowers/GraveFlowers1_Mat.GraveFlowers1_Mat"))
        (:1
          (Rendering|Material|SetMaterial Mesh 0 "/Game/Halloween/Props/Graveyard/Flowers/GraveFlowers3_Mat.GraveFlowers3_Mat"))))
    (:1
      (Components|StaticMesh|SetStaticMesh Mesh "/Game/Halloween/Props/Graveyard/Flowers/SM_Flowers_2.SM_Flowers_2")
      (switch int (Math|Random|RandomIntegerinRange 0 1)
        (:0
          (Rendering|Material|SetMaterial Mesh 0 "/Game/Halloween/Props/Graveyard/Flowers/GraveFlowers2_Mat.GraveFlowers2_Mat"))
        (:1
          (Rendering|Material|SetMaterial Mesh 0 "/Game/Halloween/Props/Graveyard/Flowers/GraveFlowers4_Mat.GraveFlowers4_Mat"))))))

(fn SetRandomCandle
  (params (Mesh :type Static%20Mesh%20Component%20Object%20Reference))
  (Transformation|SetRelativeRotation Mesh (Math|Rotator|MakeRotator 0.0 0.0 (Math|Random|RandomFloatinRange 0.0 359.0)) false false)
  (Utilities|FlowControl|Sequence
    (:then_0
      (switch int (Math|Random|RandomIntegerinRange 0 3)
        (:0
          (Components|StaticMesh|SetStaticMesh Mesh "/Game/Halloween/Props/Graveyard/SM_GraveCandle_1.SM_GraveCandle_1"))
        (:1
          (Components|StaticMesh|SetStaticMesh Mesh "/Game/Halloween/Props/Graveyard/SM_GraveCandle_2.SM_GraveCandle_2"))
        (:2
          (Components|StaticMesh|SetStaticMesh Mesh "/Game/Halloween/Props/Graveyard/SM_GraveCandle_3.SM_GraveCandle_3"))
        (:3
          (Components|StaticMesh|SetStaticMesh Mesh "/Game/Halloween/Props/Graveyard/SM_GraveCandle_4.SM_GraveCandle_4"))))
    (:then_1
      (switch int (Math|Random|RandomIntegerinRange 0 5)
        (:0
          (Rendering|Material|SetMaterial Mesh 1 "/Game/Halloween/Props/Graveyard/GraveCandleBlue_Mat.GraveCandleBlue_Mat"))
        (:1
          (Rendering|Material|SetMaterial Mesh 1 "/Game/Halloween/Props/Graveyard/GraveCandleOrange_Mat.GraveCandleOrange_Mat"))
        (:2
          (Rendering|Material|SetMaterial Mesh 1 "/Game/Halloween/Props/Graveyard/GraveCandlePink_Mat.GraveCandlePink_Mat"))
        (:3
          (Rendering|Material|SetMaterial Mesh 1 "/Game/Halloween/Props/Graveyard/GraveCandleRed_Mat.GraveCandleRed_Mat"))
        (:4
          (Rendering|Material|SetMaterial Mesh 1 "/Game/Halloween/Props/Graveyard/GraveCandleWhite_Mat.GraveCandleWhite_Mat"))
        (:5
          (Rendering|Material|SetMaterial Mesh 1 "/Game/Halloween/Props/Graveyard/GraveCandleYellow_Mat.GraveCandleYellow_Mat"))))))