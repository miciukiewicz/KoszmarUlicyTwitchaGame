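; Configurable street lamp prop with a spot light that can be lit, dark or blinking.
; The construction script swaps the mesh's second material between emissive and grey, toggles the spot light, and applies exposed color, cone and brightness settings when lit.
; It also scales the mesh uniformly and assigns or clears a light function material for blinking, so no runtime logic is needed.
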(event EventBeginPlay)

(event Collision|EventActorBeginOverlap
  (params (OtherActor :type Actor%20Object%20Reference)))

(event EventTick
  (params (DeltaSeconds :type Float%20%28single-precision%29)))

(fn ConstructionScript
  (bind _spotlight (Variables|Default|GetSpotLight))
  (bind _sm_streetlamp (Variables|Default|GetSM_StreetLamp))
  (bind _meshscale (Variables|Default|GetMeshScale))
  (bind _spotlight_2 (Variables|Default|GetSpotLight))
  (Utilities|FlowControl|Sequence
    (:then_0
      (if (Variables|Default|GetlightON)
        (Rendering|Material|SetMaterial _sm_streetlamp 1 "/Game/Halloween/Materials/Emissive/StreetLamp_Emissive_Mat.StreetLamp_Emissive_Mat")
        (Rendering|SetVisibility _spotlight true false)
        (Rendering|Components|Light|SetIntensity _spotlight (Variables|Default|GetIntensity))
        (Class|LightComponent|SetTemperature _spotlight (Variables|Default|GetTemperature))
        (Rendering|Lighting|SetInnerConeAngle _spotlight (Variables|Default|GetInner%20Cone%20Angle))
        (Rendering|Lighting|SetOuterConeAngle _spotlight (Variables|Default|GetOuter%20Cone%20Angle))
        (Rendering|Lighting|SetAttenuationRadius _spotlight (Variables|Default|GetAttentuationRadius))
        (Class|LightComponent|SetVolumetricScatteringIntensity _spotlight (Variables|Default|GetVolumetricScattering))
        (Rendering|Components|Light|SetLightColor _spotlight (Variables|Default|GetLightColor) true)
        (else
          (Rendering|Material|SetMaterial _sm_streetlamp 1 "/Game/Halloween/Materials/Simple/GreyColor_Mat.GreyColor_Mat")
          (Rendering|SetVisibility _spotlight false false))))
    (:then_1
      (Transformation|SetRelativeScale3D _sm_streetlamp (Math|Vector|MakeVector _meshscale _meshscale _meshscale)))
    (:then_2
      (if (Variables|Default|GetlightBlinking)
        (Rendering|Components|Light|SetLightFunctionMaterial _spotlight_2 "/Game/Halloween/Materials/Other/Blinking_LightFunction.Blinking_LightFunction")
        (else
          (Rendering|Components|Light|SetLightFunctionMaterial _spotlight_2 0))))))