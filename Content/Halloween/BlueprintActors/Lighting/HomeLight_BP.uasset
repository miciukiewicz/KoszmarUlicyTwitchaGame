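; HomeLight_BP is a configurable light fixture actor for the Halloween environment, set up entirely in its construction script.
; LightON swaps the mesh between on and off materials; when on, exposed variables drive intensity, temperature, color, radius, size and volumetric scattering.
; UseRectLight chooses whether the rect or point light is visible.
; The script also scales the mesh uniformly and toggles an optional blinking light function material.
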(fn ConstructionScript
  (bind _pointlight (Variables|Default|GetPointLight))
  (bind _rectlight (Variables|Default|GetRectLight))
  (bind _meshscale (Variables|Default|GetMeshScale))
  (bind _rectlight_2 (Variables|Default|GetRectLight))
  (bind _lightmesh (Variables|Default|GetLightMesh))
  (Utilities|FlowControl|Sequence
    (:then_0
      (if (Variables|Default|GetlightON)
        (Utilities|FlowControl|Sequence
          (:then_0
            (Rendering|Material|SetMaterial _lightmesh 0 "/Game/Halloween/Materials/Emissive/HomeLight_ON_Mat.HomeLight_ON_Mat")
            (Rendering|Components|Light|SetIntensity _rectlight_2 (Variables|Default|GetIntensity))
            (Class|LightComponent|SetTemperature _rectlight_2 (Variables|Default|GetTemperature))
            (Class|RectLightComponent|SetSourceWidth _rectlight_2 (Variables|Default|GetlightWidth))
            (Class|RectLightComponent|SetSourceHeight _rectlight_2 (Variables|Default|GetlightHeight))
            (Rendering|Lighting|SetAttenuationRadius _rectlight_2 (Variables|Default|GetAttentuationRadius))
            (Class|LightComponent|SetVolumetricScatteringIntensity _rectlight_2 (Variables|Default|GetVolumetricScattering))
            (Rendering|Components|Light|SetLightColor _rectlight_2 (Variables|Default|GetLightColor) true))
          (:then_1
            (if (Variables|Default|GetuseRectLight)
              (Rendering|SetVisibility _rectlight_2 true false)
              (Rendering|SetVisibility _pointlight false false)
              (else
                (Rendering|SetVisibility _pointlight true false)
                (Rendering|SetVisibility _rectlight_2 false false)))))
        (else
          (Rendering|Material|SetMaterial _lightmesh 0 "/Game/Halloween/Materials/Other/HomeLight_OFF_Mat.HomeLight_OFF_Mat")
          (Rendering|SetVisibility _rectlight_2 false false))))
    (:then_1
      (Transformation|SetRelativeScale3D _lightmesh (Math|Vector|MakeVector _meshscale _meshscale _meshscale)))
    (:then_2
      (if (Variables|Default|GetlightBlinking)
        (Rendering|Components|Light|SetLightFunctionMaterial _rectlight "/Game/Halloween/Materials/Other/Blinking_LightFunction.Blinking_LightFunction")
        (else
          (Rendering|Components|Light|SetLightFunctionMaterial _rectlight 0))))))