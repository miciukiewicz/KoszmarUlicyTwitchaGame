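; Placeable small street lamp Blueprint for the Halloween level, pairing a lamp mesh with a point light.
; The construction script uses LightON to swap the mesh's emissive or grey material and toggle the light, applying exposed intensity, temperature, color, attenuation and volumetric scattering when lit.
; It also scales the mesh uniformly and optionally assigns a blinking light function material.
; The event graph holds no runtime logic.
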(event EventBeginPlay)

(event Collision|EventActorBeginOverlap
  (params (OtherActor :type Actor%20Object%20Reference)))

(event EventTick
  (params (DeltaSeconds :type Float%20%28single-precision%29)))

(fn ConstructionScript
  (bind _sm_streetlamp (Variables|Default|GetSM_StreetLamp))
  (bind _meshscale (Variables|Default|GetMeshScale))
  (bind _pointlight (Variables|Default|GetPointLight))
  (bind _pointlight_2 (Variables|Default|GetPointLight))
  (Utilities|FlowControl|Sequence
    (:then_0
      (if (Variables|Default|GetlightON)
        (Rendering|Material|SetMaterial _sm_streetlamp 1 "/Game/Halloween/Materials/Emissive/StreetLamp_Emissive_Mat.StreetLamp_Emissive_Mat")
        (Rendering|SetVisibility _pointlight true false)
        (Rendering|Components|Light|SetIntensity _pointlight (Variables|Default|GetIntensity))
        (Class|LightComponent|SetTemperature _pointlight (Variables|Default|GetTemperature))
        (Rendering|Lighting|SetAttenuationRadius _pointlight (Variables|Default|GetAttentuationRadius))
        (Class|LightComponent|SetVolumetricScatteringIntensity _pointlight (Variables|Default|GetVolumetricScattering))
        (Rendering|Components|Light|SetLightColor _pointlight (Variables|Default|GetLightColor) true)
        (else
          (Rendering|Material|SetMaterial _sm_streetlamp 1 "/Game/Halloween/Materials/Simple/GreyColor_Mat.GreyColor_Mat")
          (Rendering|SetVisibility _pointlight false false))))
    (:then_1
      (Transformation|SetRelativeScale3D _sm_streetlamp (Math|Vector|MakeVector _meshscale _meshscale _meshscale)))
    (:then_2
      (if (Variables|Default|GetlightBlinking)
        (Rendering|Components|Light|SetLightFunctionMaterial _pointlight_2 "/Game/Halloween/Materials/Other/Blinking_LightFunction.Blinking_LightFunction")
        (else
          (Rendering|Components|Light|SetLightFunctionMaterial _pointlight_2 0))))))