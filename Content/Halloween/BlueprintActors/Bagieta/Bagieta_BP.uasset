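; Bagieta_BP is a one-shot triggered Halloween event actor that sends a Bagieta object and a chainsaw into view when the player enters its trigger.
; Overlap by the player character calls Start, which reveals both components, plays the chainsaw sound and runs a timeline sliding Bagieta along its relative Y axis.
; When the timeline finishes, a crash sound plays at Bagieta's location and the actor destroys itself after a brief delay.
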(event OnComponentBeginOverlap(Trigger)
  (params (OverlappedComponent :type Primitive%20Component%20Object%20Reference) (OtherActor :type Actor%20Object%20Reference) (OtherComp :type Primitive%20Component%20Object%20Reference) (OtherBodyIndex :type Integer) (bFromSweep :type Boolean) (SweepResult :type Hit%20Result%20Structure%20%28by%20ref%29))
  (if (== OtherActor (Game|GetPlayerCharacter 0))
    (CallFunction|Start)))

(event Custom|Start
  (Utilities|FlowControl|DoOnce false
    (:Completed
      (Rendering|SetVisibility (Variables|Default|GetBagieta) true false)
      (Audio|Components|Audio|Play (Variables|Default|GetChainsaw_Cue) 0.0)
      (bind _move (Timeline|MoveBagieta PlayFromStart)
        (:Update
          (Transformation|SetRelativeLocation (Variables|Default|GetBagieta) (Math|Vector|MakeVector 0.0 _move 0.0) false false))
        (:Finished
          (Audio|PlaySoundatLocation "/Game/Halloween/Audio/Other/CrashHit_Cue.CrashHit_Cue" (Transformation|GetWorldLocation (Variables|Default|GetBagieta)) "0, 0, 0" 1.0 1.0 0.0 0 0 0 0)
          (Utilities|FlowControl|Delay 0.2)
          (Actor|DestroyActor))))))

(fn ConstructionScript)