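; Halloween ghost AI pawn that roams the navmesh with a random material and looping sound, and catches the player.
; Patrol chains random AIMoveTo destinations with pauses, gated by SeesPlayer, while PawnSensing sightings send it toward the player.
; Overlapping CatchCollision teleports the player to a hard-coded spot and shows a timed jumpscare widget with sound.
; The catch also returns the first two ghosts to their start locations, then resumes its own patrol.
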(event OnSeePawn(PawnSensing)
  (params (Pawn :type Pawn%20Object%20Reference))
  (bind _asbp_player_character (Utilities|Casting|CastToBP_PlayerCharacter Pawn))
  (Utilities|IsValid _asbp_player_character
    (:Is%20Valid
      (bind _randomlocation (Class|NavigationSystemV1|GetRandomLocationinNavigableRadius (Transformation|GetActorLocation _asbp_player_character) 3.0 0 0))
      (AI|AIMoveTo self _randomlocation 0 2.0 false))))

(event OnComponentBeginOverlap(CatchCollision)
  (params (OverlappedComponent :type Primitive%20Component%20Object%20Reference) (OtherActor :type Actor%20Object%20Reference) (OtherComp :type Primitive%20Component%20Object%20Reference) (OtherBodyIndex :type Integer) (bFromSweep :type Boolean) (SweepResult :type Hit%20Result%20Structure%20%28by%20ref%29))
  (bind _returnvalue (Game|GetPlayerCharacter 0))
  (if (== OtherActor _returnvalue)
    (Utilities|FlowControl|DoOnce false :!label _label
      (:Completed
        (Transformation|Teleport _returnvalue "-8400.000000,-5800.000000,195.000000" "0, 0, 0")
        (Pawn|SetControlRotation (Game|GetPlayerController 0) (Math|Rotator|MakeRotator 0.0 0.0 -9e+01))
        (bind _asbp_player_character (Utilities|Casting|CastToBP_PlayerCharacter (Game|GetPlayerCharacter 0)))
        (if (not (UserInterface|Viewport|IsinViewport (Variables|/Game/Halloween/BlueprintActors/Player/BP_PlayerCharacter.BP_PlayerCharacter_C|GetGhostWidget _asbp_player_character)))
          (UserInterface|Viewport|AddtoViewport (Variables|/Game/Halloween/BlueprintActors/Player/BP_PlayerCharacter.BP_PlayerCharacter_C|GetGhostWidget _asbp_player_character) 0)
          (Utilities|FlowControl|Sequence
            (:then_0
              (bind _outactors (Actor|GetAllActorsOfClass "Ghost_BP_C"))
              (Transformation|Teleport (Utilities|Array|Get(acopy) _outactors) (Variables|Ghost_BP_C|GetstartLocation (Utilities|Array|Get(acopy) _outactors)) "0, 0, 0")
              (Transformation|Teleport (Utilities|Array|Get(acopy) _outactors 1) (Variables|Ghost_BP_C|GetstartLocation (Utilities|Array|Get(acopy) _outactors 1)) "0, 0, 0")
              (Utilities|FlowControl|Delay 1.0)
              (CallFunction|Patrol)
              (goto _label Reset))
            (:then_1
              (Utilities|FlowControl|Delay 4.0)
              (Widget|RemovefromParent (Variables|/Game/Halloween/BlueprintActors/Player/BP_PlayerCharacter.BP_PlayerCharacter_C|GetGhostWidget _asbp_player_character)))
            (:then_2
              (Audio|PlaySound2D "/Game/Halloween/Audio/Other/GhostJumpscare.GhostJumpscare" 1.0 1.0 0.0 0 0))))))))

(event Custom|Patrol
  (bind _ghostloop_cue (Variables|Default|GetGhostLoop_Cue))
  (Audio|Components|Audio|Play _ghostloop_cue (Math|Random|RandomFloatinRange 0.0 2.0))
  (Audio|Components|Audio|SetPitchMultiplier _ghostloop_cue (Math|Random|RandomFloatinRange 0.8 1.0))
  (if (not (Variables|Default|GetseesPlayer))
    (AI|AIMoveTo self (.RandomLocation (AI|Navigation|GetRandomReachablePointinRadius (Transformation|GetActorLocation) 5e+03 0 0)) 0 2.0 false
      (:OnSuccess
        (Utilities|FlowControl|Delay (Math|Random|RandomFloatinRange 2.0 5.0))
        (CallFunction|Patrol))
      (:OnFail
        (Development|PrintString "FAIL")))))

(event Custom|Teleport
  (Transformation|Teleport (Variables|Default|GetstartLocation) "0, 0, 0")
  (CallFunction|Patrol))

(event EventBeginPlay
  (Variables|Default|SetstartLocation (Transformation|GetActorLocation))
  (Rendering|Material|SetMaterial (Variables|Default|GetGhostBody) 0 (Utilities|Array|Get(acopy) (Variables|Default|GetMaterial) (Math|Random|RandomIntegerinRange 0 4)))
  (CallFunction|Patrol))

(fn ConstructionScript)