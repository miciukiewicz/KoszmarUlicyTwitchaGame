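; RoadSpline_BP is a spline actor that builds a road from a mesh laid along an editable spline.
; The construction script adds one spline mesh component per segment, bending it with the local locations and tangents of the two neighbouring points.
; Mesh, material, scale and visibility come from variables, and each segment attaches to the Scene component.
; BeginPlay does nothing.
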(event EventBeginPlay)

(fn ConstructionScript
  (bind _spline (Variables|Default|GetSpline))
  (for _index (range 0 (- (Spline|GetNumberOfSplinePoints (Variables|Default|GetSpline)) 2))
    (bind _returnvalue (AddComponent|AddSplineMeshComponent true))
    (Components|StaticMesh|SetStaticMesh _returnvalue (Variables|Default|GetMesh))
    (Rendering|Material|SetMaterial _returnvalue 0 (Variables|Default|GetMeshMaterial))
    (Transformation|SetRelativeScale3D _returnvalue (Variables|Default|GetMeshScale))
    (Transformation|AttachComponentToComponent _returnvalue (Variables|Default|GetScene) "None" "KeepRelative" "KeepRelative" "KeepRelative" true)
    (SplineMesh|SetStartandEnd _returnvalue (.Location (Spline|GetLocationandTangentatSplinePoint _spline _index "Local")) (.Tangent (Spline|GetLocationandTangentatSplinePoint _spline _index "Local")) (.Location (Spline|GetLocationandTangentatSplinePoint _spline (+ _index 1) "Local")) (.Tangent (Spline|GetLocationandTangentatSplinePoint _spline (+ _index 1) "Local")) true :!class /Script/Engine.SplineMeshComponent)
    (if (Variables|Default|GetmeshVisible)
      (Rendering|SetVisibility _returnvalue true false)
      (else
        (Rendering|SetVisibility _returnvalue false false)))))