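; Amrah is a Halloween scare actor whose Character mesh slides out and runs forward when the player enters its trigger Box.
; The one-shot trigger plays a sound cue and a timeline moving the mesh on relative Y, then starts the looping Zombie_Running animation and a second timeline on X.
; A separate KillBox overlap only prints a death message once, and the SetEnding call is left unconnected.
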(event OnComponentBeginOverlap(Box)
  (params (OverlappedComponent :type Primitive%20Component%20Object%20Reference) (OtherActor :type Actor%20Object%20Reference) (OtherComp :type Primitive%20Component%20Object%20Reference) (OtherBodyIndex :type Integer) (bFromSweep :type Boolean) (SweepResult :type Hit%20Result%20Structure%20%28by%20ref%29))
  (if (== OtherActor (Game|GetPlayerCharacter 0))
    (CallFunction|Start)))

(event OnComponentBeginOverlap(KillBox)
  (params (OverlappedComponent :type Primitive%20Component%20Object%20Reference) (OtherActor :type Actor%20Object%20Reference) (OtherComp :type Primitive%20Component%20Object%20Reference) (OtherBodyIndex :type Integer) (bFromSweep :type Boolean) (SweepResult :type Hit%20Result%20Structure%20%28by%20ref%29))
  (if (== OtherActor (Game|GetPlayerCharacter 0))
    (Utilities|FlowControl|DoOnce false
      (:Completed
        (Development|PrintString "u ded")))))

(event Custom|Start
  (bind _character (Variables|Default|GetCharacter))
  (bind _relativelocation (Variables|/Script/Engine.SceneComponent|GetRelativeLocation _character))
  (Utilities|FlowControl|DoOnce false
    (:Completed
      (Audio|Components|Audio|Play (Variables|Default|GetDemonz_CieszynkaKill_Cue) 0.0)
      (bind _move (Timeline|MoveTimeline PlayFromStart)
        (:Update
          (Transformation|SetRelativeLocation (Variables|Default|GetCharacter) (Math|Vector|MakeVector 0.0 _move 0.0) false false))
        (:Finished
          (Components|Animation|PlayAnimation (Variables|Default|GetCharacter) "/Game/Halloween/Character/Animations/Zombie_Running.Zombie_Running" true)
          (bind _move_2 (Timeline|MoveForward PlayFromStart)
            (:Update
              (Transformation|SetRelativeLocation (Variables|Default|GetCharacter) (Math|Vector|MakeVector _move_2 (.y _relativelocation) (.z _relativelocation)) false false))))))))

(fn ConstructionScript)