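; Halloween ambience actor that periodically plays the Animals_Cue sound from varying positions.
; A looping timer started on BeginPlay calls RotateAndPlay every 70 seconds.
; Each call randomizes the Cube component's relative X offset and yaw, then waits a random delay of up to 30 seconds.
; The cue then plays at the Box component's world location.
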(event Custom|RotateAndPlay
  (bind _cube (Variables|Default|GetCube))
  (Transformation|SetRelativeLocation _cube (Math|Vector|MakeVector (Math|Random|RandomFloatinRange 1.9e+04 2.3e+04) 0.0 0.0) false false)
  (Transformation|SetRelativeRotation _cube (Math|Rotator|MakeRotator 0.0 0.0 (Math|Random|RandomFloatinRange 0.0 359.0)) false false)
  (Utilities|FlowControl|Delay (Math|Random|RandomFloatinRange 0.0 3e+01))
  (Audio|PlaySoundatLocation "/Game/Halloween/Audio/Animals/Animals_Cue.Animals_Cue" (Transformation|GetWorldLocation (Variables|Default|GetBox)) "0, 0, 0" 1.0 1.0 0.0 0 0 0 0))

(event EventBeginPlay
  (Utilities|Time|SetTimerbyFunctionName 0 "RotateAndPlay" 7e+01 true))

(fn ConstructionScript)