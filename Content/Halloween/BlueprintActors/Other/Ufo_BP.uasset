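; Halloween UFO set piece that descends, reveals a cone and four Glorp components, then flies away and destroys itself.
; The saucer spins continuously; an armed player trigger starts its timeline descent from high above the placed position.
; Once landed, another trigger waits, then lerps the Glorps toward DesintegrateLocation and a linked SkeletalMesh actor toward the UFO origin.
; It hides them and reverses the same move timeline to depart.
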(event OnComponentBeginOverlap(setUfo)
  (params (OverlappedComponent :type Primitive%20Component%20Object%20Reference) (OtherActor :type Actor%20Object%20Reference) (OtherComp :type Primitive%20Component%20Object%20Reference) (OtherBodyIndex :type Integer) (bFromSweep :type Boolean) (SweepResult :type Hit%20Result%20Structure%20%28by%20ref%29))
  (if (== OtherActor (Game|GetPlayerCharacter 0))
    (Variables|Default|SetcanGo true)))

(event OnComponentBeginOverlap(startUfo)
  (params (OverlappedComponent :type Primitive%20Component%20Object%20Reference) (OtherActor :type Actor%20Object%20Reference) (OtherComp :type Primitive%20Component%20Object%20Reference) (OtherBodyIndex :type Integer) (bFromSweep :type Boolean) (SweepResult :type Hit%20Result%20Structure%20%28by%20ref%29))
  (if (== OtherActor (Game|GetPlayerCharacter 0))
    (if (Variables|Default|GetcanGo)
      (Utilities|FlowControl|DoOnce false
        (:Completed
          (CallFunction|Start))))))

(event OnComponentBeginOverlap(flyAwayUfo)
  (params (OverlappedComponent :type Primitive%20Component%20Object%20Reference) (OtherActor :type Actor%20Object%20Reference) (OtherComp :type Primitive%20Component%20Object%20Reference) (OtherBodyIndex :type Integer) (bFromSweep :type Boolean) (SweepResult :type Hit%20Result%20Structure%20%28by%20ref%29))
  (if (== OtherActor (Game|GetPlayerCharacter 0))
    (Utilities|FlowControl|Delay 5.0)
    (if (Variables|Default|GetufoLanded)
      (Utilities|FlowControl|DoOnce false
        (:Completed
          (CallFunction|FlyAway))))))

(event Custom|Rotate
  (bind _rotate (Timeline|Timeline PlayFromStart)
    (:Update
      (Transformation|SetRelativeRotation (Variables|Default|GetSM_Ufo) (Math|Rotator|MakeRotator 0.0 0.0 _rotate) false false))
    (:Finished
      (CallFunction|Rotate))))

(event Custom|Start
  (Audio|Components|Audio|Play (Variables|Default|GetUfoLoop_Cue) 0.0)
  (bind _move (Timeline|MoveUfo PlayFromStart)
    (:Update
      (Transformation|SetWorldLocation (Variables|Default|GetSM_Ufo) (Math|Vector|Lerp(Vector) (Variables|Default|GetstartLocation) (Variables|Default|GetlandLocation) _move) false false))
    (:Finished
      (if (Variables|Default|GetufoAway)
        (Utilities|FlowControl|Delay 1.0)
        (Actor|DestroyActor)
        (else
          (Rendering|SetVisibility (Variables|Default|GetSM_UfoCone) true false)
          (Variables|Default|SetufoLanded true))))))

(event Custom|FlyAway
  (bind _move (Timeline|DesintegrateTimeline PlayFromStart)
    (:Update
      (CallFunction|Desintegrate (Variables|Default|GetGlorp1) _move)
      (CallFunction|Desintegrate (Variables|Default|GetGlorp2) _move)
      (CallFunction|Desintegrate (Variables|Default|GetGlorp3) _move)
      (CallFunction|Desintegrate (Variables|Default|GetGlorp4) _move (Variables|Default|GetSkeletalMesh)))
    (:Finished
      (Rendering|SetVisibility (Variables|Default|GetGlorp2) false false)
      (Rendering|SetActorHiddenInGame (Variables|Default|GetSkeletalMesh) true)
      (Variables|Default|SetufoAway true)
      (bind _move_2 (Timeline|MoveUfo ReverseFromEnd)
        (:Update
          (Transformation|SetWorldLocation (Variables|Default|GetSM_Ufo) (Math|Vector|Lerp(Vector) (Variables|Default|GetstartLocation) (Variables|Default|GetlandLocation) _move_2) false false))
        (:Finished
          (if (Variables|Default|GetufoAway)
            (Utilities|FlowControl|Delay 1.0)
            (Actor|DestroyActor)
            (else
              (Rendering|SetVisibility (Variables|Default|GetSM_UfoCone) true false)
              (Variables|Default|SetufoLanded true))))))))

(event EventBeginPlay
  (CallFunction|Rotate)
  (bind _output_get (Variables|Default|SetlandLocation (Transformation|GetWorldLocation (Variables|Default|GetSM_Ufo))))
  (Variables|Default|SetstartLocation (+ _output_get "0.000000,0.000000,50000.000000"))
  (Transformation|SetWorldLocation (Variables|Default|GetSM_Ufo) (Variables|Default|GetstartLocation) false false))

(fn ConstructionScript)

(fn Desintegrate
  (params (Target :type Scene%20Component%20Object%20Reference) (Alpha :type Float%20%28single-precision%29) (SkeletalMesh :type Actor%20Object%20Reference))
  (Transformation|SetRelativeLocation Target (Math|Vector|Lerp(Vector) (Variables|/Script/Engine.SceneComponent|GetRelativeLocation Target) (Variables|/Script/Engine.SceneComponent|GetRelativeLocation (Variables|Default|GetDesintegrateLocation)) Alpha) false false)
  (Utilities|IsValid SkeletalMesh
    (:Is%20Valid
      (Transformation|SetActorLocation SkeletalMesh (Math|Vector|Lerp(Vector) (Transformation|GetActorLocation SkeletalMesh) (Transformation|GetActorLocation) Alpha) false false))))