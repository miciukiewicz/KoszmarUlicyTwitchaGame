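; Car alarm actor that goes off once when the player character enters its trigger box.
; The overlap plays the alarm audio and starts a looping timer that flashes four components by toggling their visibility.
; A fixed delay then clears the timer, ending the blinking after a few seconds.
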(event OnComponentBeginOverlap(Box)
  (params (OverlappedComponent :type Primitive%20Component%20Object%20Reference) (OtherActor :type Actor%20Object%20Reference) (OtherComp :type Primitive%20Component%20Object%20Reference) (OtherBodyIndex :type Integer) (bFromSweep :type Boolean) (SweepResult :type Hit%20Result%20Structure%20%28by%20ref%29))
  (if (== OtherActor (Game|GetPlayerCharacter 0))
    (Utilities|FlowControl|DoOnce false
      (:Completed
        (Audio|Components|Audio|Play (Variables|Default|GetCarAlarm_Cue) 0.0)
        (CallFunction|Start)
        (Utilities|FlowControl|Delay 7.8)
        (CallFunction|Stop)))))

(event Custom|Blink
  (bind _l4 (Variables|Default|GetL4))
  (Rendering|SetVisibility _l4 true false)
  (Utilities|FlowControl|Delay 0.5)
  (Rendering|SetVisibility _l4 false false))

(event Custom|Start
  (bind _returnvalue (Utilities|Time|SetTimerbyFunctionName 0 "Blink" 1.0 true)))

(event Custom|Stop
  (Utilities|Time|ClearandInvalidateTimerbyHandle (stale Custom|Start _returnvalue)))

(event EventBeginPlay)

(event Collision|EventActorBeginOverlap
  (params (OtherActor :type Actor%20Object%20Reference)))

(event EventTick
  (params (DeltaSeconds :type Float%20%28single-precision%29)))

(fn ConstructionScript)