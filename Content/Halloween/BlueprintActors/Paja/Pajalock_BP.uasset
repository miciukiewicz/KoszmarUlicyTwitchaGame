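; Halloween Pajalock actor that runs a one-time scripted car scene, with trigger boxes for an audio cue and a kill zone.
; MoveCar reveals the Honda, disables player input, teleports the player to a fixed spot and slides the car along X with a timeline.
; CueBox plays PajalockCue once on player overlap.
; KillBox only prints a death message, and a SetEnding call is left unconnected.
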(event OnComponentBeginOverlap(KillBox)
  (params (OverlappedComponent :type Primitive%20Component%20Object%20Reference) (OtherActor :type Actor%20Object%20Reference) (OtherComp :type Primitive%20Component%20Object%20Reference) (OtherBodyIndex :type Integer) (bFromSweep :type Boolean) (SweepResult :type Hit%20Result%20Structure%20%28by%20ref%29))
  (if (== OtherActor (Game|GetPlayerCharacter 0))
    (Utilities|FlowControl|DoOnce false
      (:Completed
        (Development|PrintString "u ded")))))

(event OnComponentBeginOverlap(CueBox)
  (params (OverlappedComponent :type Primitive%20Component%20Object%20Reference) (OtherActor :type Actor%20Object%20Reference) (OtherComp :type Primitive%20Component%20Object%20Reference) (OtherBodyIndex :type Integer) (bFromSweep :type Boolean) (SweepResult :type Hit%20Result%20Structure%20%28by%20ref%29))
  (if (== OtherActor (Game|GetPlayerCharacter 0))
    (Utilities|FlowControl|DoOnce false
      (:Completed
        (Audio|Components|Audio|Play (Variables|Default|GetPajalock_Cue) 0.0)))))

(event Custom|MoveCar
  (bind _returnvalue (Game|GetPlayerController 0))
  (bind _returnvalue_2 (Game|GetPlayerCharacter 0))
  (Utilities|FlowControl|DoOnce false
    (:Completed
      (Rendering|SetVisibility (Variables|Default|GetHonda) true false)
      (Pawn|SetControlRotation _returnvalue (Math|Rotator|MakeRotator 0.0 0.0 0.0))
      (Input|DisableInput _returnvalue_2 _returnvalue)
      (Transformation|Teleport _returnvalue_2 "1240.000000,8420.000000,190.000000" "0, 0, 0")
      (bind _move (Timeline|Move PlayFromStart)
        (:Update
          (Transformation|SetRelativeLocation (Variables|Default|GetHonda) (Math|Vector|MakeVector _move 0.0 0.0) false false))))))

(event EventBeginPlay)

(fn ConstructionScript)