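; ExampleBuildingSpawner_BP is an example actor in DynamicGrassLite that spawns a building when its Action event fires.
; It traces vertically on the Visibility channel at a fixed sideways offset from itself to find the surface.
; It then always spawns a slightly enlarged ExampleSpawnedObject_Building_BP at the hit location, aligned to the surface normal.
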(event EventAction
  (bind _returnvalue (Transformation|GetActorRightVector))
  (bind _returnvalue_2 (Transformation|GetActorLocation))
  (bind _returnvalue_3 (* _returnvalue -777.0))
  (bind _returnvalue_4 (+ _returnvalue_2 _returnvalue_3))
  (bind _outhit (Collision|LineTraceByChannel (+ _returnvalue_4 "0, 0,5000.000000") (- _returnvalue_4 "0, 0,5000.000000") "TraceTypeQuery1" false 0 "None"))
  (Game|SpawnActorfromClass "/Game/DynamicGrassLite/Blueprints/InternalLogic/ExampleSpawnedObject_Building_BP.ExampleSpawnedObject_Building_BP_C" (Math|Transform|MakeTransform (.Location (Collision|BreakHitResult _outhit)) (Math|Rotator|MakeRotfromZ (.Normal (Collision|BreakHitResult _outhit))) "1.200000,1.200000,1.200000") "AlwaysSpawn" "OverrideRootScale" 0 0))

(fn ConstructionScript
  (|CallParentFunction))